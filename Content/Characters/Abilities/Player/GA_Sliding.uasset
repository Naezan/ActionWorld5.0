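; Player slide gameplay ability that flags PlayerBase as sliding and propels the character forward.
; After an entry check, it lowers the walkable floor angle, applies an additive constant root-motion force and chains start and loop montages.
; Near-zero speed or another input press plays the end montage, and ending the ability restores movement settings and clears the flag.
; The slope-friction helper AddSlidingForce and the CheckMovement montage-stop handler are not hooked up here.
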(event Custom|CheckMovement
  (params (DeltaSeconds :type Float%20%28single-precision%29) (OldLocation :type Vector) (OldVelocity :type Vector))
  (bind _returnvalue (Class|ActionGameplayAbility|GetActionCharacterfromActorInfo))
  ;[1 1 1] 플레이어의 상태가 변하면 에니메이션을 멈춥니다
  (if (or (> (Math|Vector|VectorLength OldVelocity) 0.0) (Variables|/Script/Engine.Character|GetbIsCrouched _returnvalue))
    (EventDispatchers|UnbindallEventsfromOnCharacterMovementUpdated _returnvalue)
    (Animation|StopAnimMontage _returnvalue (Variables|Default|GetMontage%20to%20Play))))

(event Ability|EventActivateAbility
  (bind _returnvalue (Class|ActionGameplayAbility|GetActionCharacterfromActorInfo))
  (bind (_charactermovement _returnvalue_2) (|CollapseGraph_0 _returnvalue))
  (if _returnvalue_2
    (bind _asplayer_base (Utilities|Casting|CastToPlayerBase (Class|ActionGameplayAbility|GetActionCharacterfromActorInfo)))
    (Variables|/Script/ActionWorldRPG.PlayerBase|SetbIsSliding _asplayer_base true)
    (Pawn|Components|CharacterMovement|SetWalkableFloorAngle _charactermovement 1.0)
    (|PlayMontageandWaitProxy "None" "/Game/Assets/UTA_UltimateAnimation/Sliding/MM_Sliding_Start_Retargeted_Montage.MM_Sliding_Start_Retargeted_Montage" 1.0 "None" true 1.0 0.33
      (:then
        (Variables|Default|SetDirection (Transformation|GetActorForwardVector (Class|ActionGameplayAbility|GetActionCharacterfromActorInfo)))
        (Ability|Tasks|ApplyRootMotionConstantForce "None" (Variables|Default|GetDirection) (Variables|Default|GetStrength) (Variables|Default|GetRootMotionDuration) true 0 "ClampVelocity" "0, 0, 0" 1e+03))
      (:OnCompleted
        (Ability|EndAbility :!label _label))
      (:OnBlendOut
        (|PlayMontageandWaitProxy "None" "/Game/Assets/UTA_UltimateAnimation/Sliding/MM_Sliding_Loop_Retargeted_Montage.MM_Sliding_Loop_Retargeted_Montage" 1.0 "None" true 1.0 0.0
          (:then
            (|WaitforZeroSpeed "None"
              (:then
                ;[1 1 1] 슬라이딩키를 다시 누른경우
                (Ability|Tasks|WaitInputPress false
                  (:OnPress
                    _)))
              (:OnNearToZero
                _))
            (|PlayMontageandWaitProxy "None" "/Game/Assets/UTA_UltimateAnimation/Sliding/MM_Sliding_End_Retargeted_Montage.MM_Sliding_End_Retargeted_Montage" 1.0 "None" true 1.0 0.0
              (:OnCompleted
                _)
              (:OnBlendOut
                _)
              (:OnInterrupted
                _)
              (:OnCancelled
                _))
            (Ability|EndAbility))
          (:OnCompleted
            (Ability|EndAbility :!label _label_2))
          (:OnBlendOut
            (goto _label_2))
          (:OnInterrupted
            (goto _label_2))
          (:OnCancelled
            (goto _label_2))))
      (:OnInterrupted
        (goto _label))
      (:OnCancelled
        (goto _label)))
    (else
      (Ability|EndAbility))))

(event Ability|EventOnEndAbility
  (params (bWasCancelled :type Boolean))
  (bind _returnvalue (Class|ActionGameplayAbility|GetActionCharacterfromActorInfo))
  (bind _charactermovement (Variables|/Script/Engine.Character|GetCharacterMovement _returnvalue))
  (Pawn|Components|CharacterMovement|SetWalkableFloorAngle (Variables|/Script/Engine.Character|GetCharacterMovement (Class|ActionGameplayAbility|GetActionCharacterfromActorInfo)) 45.0)
  (Variables|/Script/Engine.CharacterMovementComponent|SetGroundFriction _charactermovement 4.0)
  (Variables|/Script/Engine.CharacterMovementComponent|SetBrakingDecelerationWalking _charactermovement 1e+03)
  (bind _asplayer_base (Utilities|Casting|CastToPlayerBase (Class|ActionGameplayAbility|GetActionCharacterfromActorInfo)))
  (Variables|/Script/ActionWorldRPG.PlayerBase|SetbIsSliding _asplayer_base false))

(fn AddSlidingForce
  (bind _returnvalue (Class|ActionGameplayAbility|GetActionCharacterfromActorInfo))
  (bind _returnvalue_2 (Class|ActionGameplayAbility|GetActionCharacterfromActorInfo))
  (bind _charactermovement (Variables|/Script/Engine.Character|GetCharacterMovement _returnvalue))
  (bind _charactermovement_2 (Variables|/Script/Engine.Character|GetCharacterMovement _returnvalue_2))
  (bind _currentfloor (Variables|/Script/Engine.CharacterMovementComponent|GetCurrentFloor _charactermovement))
  (bind _hitresult (Utilities|Struct|BreakFindFloorResult _currentfloor))
  (bind _impactnormal (Collision|BreakHitResult _hitresult))
  (bind _returnvalue_3 (Math|Vector|DotProduct _impactnormal "0, 0,1.000000"))
  (bind _returnvalue_4 (Class|KismetMathLibrary|DegAcos _returnvalue_3))
  (bind _output_get (Variables|Default|SetImpact%20Normal _impactnormal))
  (if (== _returnvalue_4 0.0)
    (Variables|Default|SetXForce 1.0)
    (Variables|Default|SetYForce 1.0)
    (else
      (Variables|Default|SetXForce (* _returnvalue_4 (.x _output_get)))
      (Variables|Default|SetYForce (* _returnvalue_4 (.y _output_get)))))
  (Utilities|FlowControl|Sequence
    (:then_0
      (Variables|/Script/Engine.CharacterMovementComponent|SetGroundFriction _charactermovement_2 1.0)
      (Variables|/Script/Engine.CharacterMovementComponent|SetBrakingDecelerationWalking _charactermovement_2 1e+02))
    (:then_1
      (return))))