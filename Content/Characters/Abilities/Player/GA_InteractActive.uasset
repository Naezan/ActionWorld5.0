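; Player gameplay ability that performs a timed hold or instant interaction on the hit actor supplied by the activating event's target data.
; It validates the single hit for immediate-interaction support and range, then queries the target's interaction duration.
; Interface messages register the interacter and bracket a WaitDelay with pre/post interact calls, skipping the wait at zero duration.
; Releasing input early cancels the ability, and any cancellation with a valid target sends it CancelInteraction.
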(event Ability|EventOnEndAbility
  (params (bWasCancelled :type Boolean))
  (bind _event_data_target_data (Variables|Default|GetEvent%20Data%20Target%20Data))
  (bind _returnvalue (Ability|TargetData|GetHitResultfromTargetData _event_data_target_data))
  (if bWasCancelled
    (if (and (Ability|TargetData|TargetDataHasHitResult _event_data_target_data) (Utilities|IsValid (.hitactor _returnvalue)))
      (Class|InteractInterface|CancelInteraction(Message) (.hitactor _returnvalue) (.hitcomponent _returnvalue)))))

(event Ability|EventActivateAbilityFromEvent
  (params (EventData :type Gameplay%20Event%20Data%20Structure%20%28by%20ref%29))
  (bind _returnvalue (Ability|GetAvatarActorfromActorInfo))
  (bind _isvalid (CallFunction|ValidateTarget (.targetdata EventData)))
  (if _isvalid
    (bind _output_get (Variables|Default|SetEvent%20Data%20Target%20Data (.targetdata EventData)))
    (bind _returnvalue_2 (Class|InteractInterface|GetInteractionDuration(Message) (.hitactor (Ability|TargetData|GetHitResultfromTargetData _output_get)) (.hitcomponent (Ability|TargetData|GetHitResultfromTargetData _output_get))))
    (Variables|Default|SetInteractionDuration _returnvalue_2)
    (if (> (Variables|Default|GetInteractionDuration) 0.0)
      (bind _asynctaskproxy (Ability|Tasks|WaitInputRelease false)
        (:then
          (Variables|Default|SetWait%20Input%20ReleaseAsync%20Task _asynctaskproxy)
          (Variables|Default|SetIs%20Interacting true :!label _label)
          ;[1 1 1] 타겟 데이터의 함수 실행
          (Class|InteractInterface|RegisterInteracter(Message) (.hitactor (Ability|TargetData|GetHitResultfromTargetData (Variables|Default|GetEvent%20Data%20Target%20Data))) (.hitcomponent (Ability|TargetData|GetHitResultfromTargetData (Variables|Default|GetEvent%20Data%20Target%20Data))) _returnvalue)
          (Class|InteractInterface|PreInteract(Message) (.hitactor (Ability|TargetData|GetHitResultfromTargetData (Variables|Default|GetEvent%20Data%20Target%20Data))) _returnvalue (.hitcomponent (Ability|TargetData|GetHitResultfromTargetData (Variables|Default|GetEvent%20Data%20Target%20Data))))
          (if (> (Variables|Default|GetInteractionDuration) 0.0) ; WaitDelay will not work with 0 duration
            (bind _asynctaskproxy_2 (Ability|Tasks|WaitDelay (Variables|Default|GetInteractionDuration))
              (:then
                (Variables|Default|SetWaitDelayTask _asynctaskproxy_2))
              (:OnFinish
                ;[1 1 1] 입력뒤에 실행할 타겟함수
                (Class|InteractInterface|PostInteract(Message) (.hitactor (Ability|TargetData|GetHitResultfromTargetData (Variables|Default|GetEvent%20Data%20Target%20Data))) _returnvalue (.hitcomponent (Ability|TargetData|GetHitResultfromTargetData (Variables|Default|GetEvent%20Data%20Target%20Data))) :!label _label_2)
                (Class|InteractInterface|UnregisterInteracter(Message) (.hitactor (Ability|TargetData|GetHitResultfromTargetData (Variables|Default|GetEvent%20Data%20Target%20Data))) (.hitcomponent (Ability|TargetData|GetHitResultfromTargetData (Variables|Default|GetEvent%20Data%20Target%20Data))) _returnvalue)
                (Ability|EndAbility)))
            (else
              (goto _label_2))))
        (:OnRelease
          (if (Variables|Default|GetIs%20Interacting)
            (Ability|CancelAbility)
            (else
              (Ability|EndAbility)))))
      (else
        (goto _label)))
    (else
      (Ability|CancelAbility))))

(fn ValidateTarget
  (params (TargetData :type Gameplay%20Ability%20Target%20Data%20Handle%20Structure))
  (bind _returnvalue (Ability|TargetData|GetHitResultfromTargetData TargetData))
  (if true
    (bind _returnvalue_2 (Class|InteractInterface|IsImmediateInteraction(Message) (.hitactor _returnvalue) (.hitcomponent _returnvalue)))
    (return (Math|Boolean|ANDBoolean _returnvalue_2 (== (Ability|TargetData|GetDataCountfromTargetData TargetData) 1) (Ability|TargetData|TargetDataHasHitResult TargetData) (Utilities|IsValid (.hitactor _returnvalue)) (Utilities|IsValid (.hitcomponent _returnvalue)) (<= (Class|KismetMathLibrary|VectorDistanceSquared (Transformation|GetActorLocation (Ability|GetAvatarActorfromActorInfo)) (Transformation|GetWorldLocation (.hitcomponent _returnvalue))) (Math|Float|Square (Variables|Default|GetMax%20Distance%20to%20Target)))))))