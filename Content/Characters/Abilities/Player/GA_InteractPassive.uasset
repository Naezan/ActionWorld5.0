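; Passive player Gameplay Ability that detects interactable targets and turns input presses into interaction events.
; An async task searches every frame and stores the found target's data, then waits for an input press.
; A press waits until the blocking tag is absent, then sends an Ability.Interaction gameplay event carrying that target data.
; Losing the target ends the pending input and tag tasks and clears the data.
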(event Custom|InteractionProccess
  (bind _asynctaskproxy (Ability|Tasks|WaitInputPress false)
    (:then
      (Variables|Default|SetWait%20InputPressAsync%20Task _asynctaskproxy))
    (:OnPress
      (bind _asynctaskproxy_2 (Ability|Tasks|WaitGameplayTagRemove (Variables|Default|GetActiveBlockedTag) 0 true) ; If tag is not present, it will broadcast immediately.
        (:then
          (Variables|Default|SetWait%20Gameplay%20Tag%20Remove%20Async%20Task _asynctaskproxy_2))
        (:Removed
          (bind _wait_inputpressasync_task (Variables|Default|GetWait%20InputPressAsync%20Task)
            (:then
              (GameplayTasks|EndTask _wait_inputpressasync_task))
            (:else
              _))
          (Ability|SendGameplayEvent "(TagName=\"Ability.Interaction\")" (Utilities|Struct|MakeGameplayEventData "(TagName=\"\")" 0 0 0 0 "()" "(GameplayTags=)" "(GameplayTags=)" 0.0 (Variables|Default|GetTrace%20Target%20Data))))))))

(event Ability|EventActivateAbility
  (bind (_asynctaskproxy _data) (|WaitforInteractableTarget "None" "(Name=\"InteractTrace\")" 2e+02 0.1 (Variables|Default|GetShowDebugTrace)) ; 매 프레임마다 비동기적으로 타겟 찾기
    (:then
      (Variables|Default|SetWait%20Interactable%20TargetAsync%20Task _asynctaskproxy))
    (:FoundNewInteractableTarget
      (Variables|Default|SetTrace%20Target%20Data _data)
      (CallFunction|InteractionProccess))
    (:LostInteractableTarget
      (bind _wait_inputpressasync_task (Variables|Default|GetWait%20InputPressAsync%20Task)
        (:then
          (GameplayTasks|EndTask _wait_inputpressasync_task))
        (:else
          _))
      (bind _wait_gameplay_tag_remove_async_task (Variables|Default|GetWait%20Gameplay%20Tag%20Remove%20Async%20Task)
        (:then
          (GameplayTasks|EndTask _wait_gameplay_tag_remove_async_task))
        (:else
          _))
      (Class|ActionBlueprintFunctionLibrary|ClearTargetData (Variables|Default|GetTrace%20Target%20Data)))))