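; GA_NextWeapon is a player gameplay ability that switches BP_Player to its next weapon.
; Activation is allowed only when the player has more than one weapon.
; It calls NextWeapon on the avatar, applies the GE_WeaponChangeDelayTime effect to the owner, then ends immediately.
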(event Ability|EventActivateAbility
  (bind _asbp_player (Utilities|Casting|CastToBP_Player (Ability|GetAvatarActorfromActorInfo)))
  (bind _output_get (Variables|Default|SetOwningPlayer _asbp_player))
  (Class|PlayerBase|NextWeapon _output_get)
  (Ability|ApplyGameplayEffectToOwner "/Game/Characters/Abilities/Player/GE_WeaponChangeDelayTime.GE_WeaponChangeDelayTime_C")
  (Ability|EndAbility))

(fn K2CanActivateAbility
  (params (ActorInfo :type Gameplay%20Ability%20Actor%20Info%20Structure) (Handle :type Gameplay%20Ability%20Spec%20Handle%20Structure))
  (bind _asbp_player (Utilities|Casting|CastToBP_Player (.avataractor ActorInfo)))
  (if (> (Class|PlayerBase|GetNumWeapons _asbp_player) 1)
    (return "" true)
    (else
      (return "" false))))