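; BP_Player is the player character, handling Enhanced Input for movement, camera look, jump, crouch toggle and a faster-speed jog override.
; On BeginPlay it snaps to the floor using a temporarily enlarged step height, enters Walking and adds the IM_Controls mapping context.
; Forward and right inputs feed GetMovementSpeed, which clamps low combined magnitudes as one vector to avoid speeds between walk and jog, then move relative to control yaw.
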(event Input|EnhancedActionEvents|EnhancedInputActionIA_MoveForward
  (params (ActionValue :type Float%20%28double-precision%29) (ElapsedSeconds :type Float%20%28double-precision%29) (TriggeredSeconds :type Float%20%28double-precision%29) (InputAction :type Input%20Action%20Object%20Reference :default "/Game/Input/IA_MoveForward.IA_MoveForward"))
  ;[1 1 1] 입력
  (:Triggered
    (goto _label Triggered))
  (:Started
    (Utilities|MoveForwardAction ActionValue TriggeredSeconds :!label _label))
  (:Completed
    (goto _label Finished)))

(event Input|EnhancedActionEvents|EnhancedInputActionIA_MoveRight
  (params (ActionValue :type Float%20%28double-precision%29) (ElapsedSeconds :type Float%20%28double-precision%29) (TriggeredSeconds :type Float%20%28double-precision%29) (InputAction :type Input%20Action%20Object%20Reference :default "/Game/Input/IA_MoveRight.IA_MoveRight"))
  ;[1 1 1] 입력
  (:Triggered
    (goto _label Triggered))
  (:Started
    (Utilities|MoveRightAction ActionValue TriggeredSeconds :!label _label))
  (:Completed
    (goto _label Finished)))

(event Input|EnhancedActionEvents|EnhancedInputActionIA_JogOverride
  (params (ActionValue :type Boolean) (ElapsedSeconds :type Float%20%28double-precision%29) (TriggeredSeconds :type Float%20%28double-precision%29) (InputAction :type Input%20Action%20Object%20Reference :default "/Game/Input/IA_JogOverride.IA_JogOverride"))
  ;[1 1 1] 입력
  (:Triggered
    (goto _label Triggered))
  (:Started
    (Utilities|JogOverrideAction :!label _label))
  (:Completed
    (goto _label Finished)))

(event Input|EnhancedActionEvents|EnhancedInputActionIA_LookUp
  (params (ActionValue :type Float%20%28double-precision%29) (ElapsedSeconds :type Float%20%28double-precision%29) (TriggeredSeconds :type Float%20%28double-precision%29) (InputAction :type Input%20Action%20Object%20Reference :default "/Game/Input/IA_LookUp.IA_LookUp"))
  ;[1 1 1] 입력
  ;;[1 1 1] 마우스
  (:Triggered
    (CallFunction|HandleLookUpInput ActionValue)))

(event Input|EnhancedActionEvents|EnhancedInputActionIA_Turn
  (params (ActionValue :type Float%20%28double-precision%29) (ElapsedSeconds :type Float%20%28double-precision%29) (TriggeredSeconds :type Float%20%28double-precision%29) (InputAction :type Input%20Action%20Object%20Reference :default "/Game/Input/IA_Turn.IA_Turn"))
  ;[1 1 1] 입력
  ;;[1 1 1] 마우스
  (:Triggered
    (CallFunction|HandleTurnInput ActionValue)))

(event Input|EnhancedActionEvents|EnhancedInputActionIA_Jump
  (params (ActionValue :type Boolean) (ElapsedSeconds :type Float%20%28double-precision%29) (TriggeredSeconds :type Float%20%28double-precision%29) (InputAction :type Input%20Action%20Object%20Reference :default "/Game/Input/IA_Jump.IA_Jump"))
  ;[1 1 1] 입력
  (:Triggered
    (Character|Jump))
  (:Completed
    (Character|StopJumping)))

(event Input|EnhancedActionEvents|EnhancedInputActionIA_Crouch
  (params (ActionValue :type Boolean) (ElapsedSeconds :type Float%20%28double-precision%29) (TriggeredSeconds :type Float%20%28double-precision%29) (InputAction :type Input%20Action%20Object%20Reference :default "/Game/Input/IA_Crouch.IA_Crouch"))
  ;[1 1 1] 입력
  (:Triggered
    (bind _isa (Utilities|FlowControl|FlipFlop)
      (:A
        (Character|Crouch))
      (:B
        (Character|UnCrouch)))))

(event EventBeginPlay
  (입력|MovetoFloor)
  (Pawn|Components|CharacterMovement|SetMovementMode (Variables|Character|GetCharacterMovement) "MOVE_Walking" 0)
  (Input|AddMappingContext (PlayerController|LocalPlayerSubsystems|GetEnhancedInputLocalPlayerSubsystem (Game|GetPlayerController 0)) "/Game/Input/IM_Controls.IM_Controls" 0 "(bIgnoreAllPressedKeysUntilRelease=True,bForceImmediately=False)"))

(event EventPossessed
  (params (NewController :type Controller%20Object%20Reference))
  (Utilities|Casting|CastToPlayerController NewController))

(fn ConstructionScript)

(fn MovetoFloor
  (bind _capsulecomponent (Variables|Default|GetCapsuleComponent))
  (bind _charactermovement (Variables|Character|GetCharacterMovement))
  (bind _returnvalue (Transformation|GetWorldLocation _capsulecomponent))
  (bind _floorresult (Pawn|Components|CharacterMovement|FindFloor _charactermovement _returnvalue))
  (LocalVariables|SetInitialStepHeight (Variables|/Script/Engine.CharacterMovementComponent|GetMaxStepHeight (Variables|Character|GetCharacterMovement)))
  (Variables|/Script/Engine.CharacterMovementComponent|SetMaxStepHeight (Variables|Character|GetCharacterMovement) (LocalVariables|GetLargeStepHeight))
  (if (.bblockinghit _floorresult)
    (Transformation|Teleport (+ _returnvalue (Math|Vector|MakeVector 0.0 0.0 (.floordist _floorresult))) (Transformation|GetActorRotation))
    (Variables|/Script/Engine.CharacterMovementComponent|SetMaxStepHeight (Variables|Character|GetCharacterMovement) (LocalVariables|GetInitialStepHeight))))

(fn HandleLookUpInput
  (params (InputValue :type Float%20%28double-precision%29))
  (Pawn|Input|AddControllerPitchInput InputValue))

(fn HandleTurnInput
  (params (InputValue :type Float%20%28double-precision%29))
  (Pawn|Input|AddControllerYawInput InputValue))

(fn HandleForwardInput
  (params (InputValue :type Float%20%28double-precision%29))
  (Pawn|Input|AddMovementInput (Math|Vector|GetForwardVector (Math|Rotator|MakeRotator 0.0 0.0 (.yaw (Pawn|GetControlRotation :!class /Script/Engine.Pawn)))) InputValue false))

(fn GetMovementSpeed
  (bind _returnvalue (Math|Float|MakeLiteralFloat 0.586))
  (bind _ia_moveforward_action_value (Variables|입력|GetIA_MoveForward_Action%20Value))
  (bind _ia_moveright_action_value (Variables|입력|GetIA_MoveRight_Action%20Value))
  (bind _returnvalue_2 (Math|Vector|MakeVector _ia_moveforward_action_value _ia_moveright_action_value 0.0))
  (bind _returnvalue_3 (Math|Float|Absolute(Float) _returnvalue))
  (bind _returnvalue_4 (Math|Vector|VectorLength _returnvalue_2))
  (bind _returnvalue_5 (Math|Vector|ClampVectorSize _returnvalue_2 0.287 0.332))
  (bind _returnvalue_6 (Math|Float|Absolute(Float) _returnvalue_4))
  (bind _returnvalue_7 (< _returnvalue_6 _returnvalue_3))
  (bind _returnvalue_8 (Math|Vector|SelectVector _returnvalue_5 _returnvalue_2 _returnvalue_7))
  ;[1 1 1] Keep character from moving too slowly and from having speeds too fast for walk but too slow for jog.   Doing this with both values at the same time to make a vector rather than individually for each axis because this creates proper vector length.  Doing it individually creates a square "deadzone" that has a longer vector on the diagonals
  (return (.x _returnvalue_8) (.y _returnvalue_8)))

(fn HandleRightwardInput
  (params (InputValue :type Float%20%28double-precision%29))
  (Pawn|Input|AddMovementInput (Math|Vector|GetRightVector (Math|Rotator|MakeRotator 0.0 0.0 (.yaw (Pawn|GetControlRotation :!class /Script/Engine.Pawn)))) InputValue false))