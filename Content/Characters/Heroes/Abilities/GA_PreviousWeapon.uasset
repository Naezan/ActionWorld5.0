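; Gameplay ability that switches the hero to the previous weapon.
; Activation is allowed only when the BP_Player avatar carries more than one weapon.
; It calls PreviousWeapon, applies GE_WeaponChangeDelayTime to the owner and ends at once.
; That effect's tag lasts about a second beyond the equip montage, holding off CurrentWeapon replication during the change.
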(event Ability|EventActivateAbility
  (bind _asbp_player (Utilities|Casting|CastToBP_Player (Ability|GetAvatarActorfromActorInfo)))
  (bind _output_get (Variables|Default|SetOwningHero _asbp_player))
  (Class|PlayerBase|PreviousWeapon _output_get)
  (Ability|ApplyGameplayEffectToOwner "/Game/Characters/Heroes/Abilities/GE_WeaponChangeDelayTime.GE_WeaponChangeDelayTime_C") ; Equip montages are about 0.5s, this tag will last 1.5s. This gives us 1s of extra time that the CurrentWeapon is not allowed to replicate.
  (Ability|EndAbility))

(fn K2CanActivateAbility
  (params (ActorInfo :type Gameplay%20Ability%20Actor%20Info%20Structure) (Handle :type Gameplay%20Ability%20Spec%20Handle%20Structure))
  (bind _asbp_player (Utilities|Casting|CastToBP_Player (.avataractor ActorInfo)))
  (if (> (Class|PlayerBase|GetNumWeapons _asbp_player) 1)
    (return "" true)
    (else
      (return "" false))))