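; Primary fire ability for the rifle, driving GA_RiflePrimaryInstant according to the weapon's semi-auto, full-auto or burst fire mode.
; The first shot batch-activates the instant ability in one RPC.
; Full-auto and burst then call FireBullet on its cached instance at timed intervals, rechecking cost, until release, burst end or empty clip.
; CheckCost tests clip or infinite ammo and triggers reload by tag when it fails while inactive.
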(event Ability|EventActivateAbility
  (bind _sourceweapon (Variables|Default|GetSourceWeapon))
  (bind _firemode (Variables|/Script/ActionWorldRPG.WeaponBase|GetFireMode _sourceweapon))
  (Utilities|CheckandSetUpCacheables)
  (Ability|Tasks|WaitDelay 0.03
    (:OnFinish
      ;[1 1 1] 반자동
      (if (== _firemode "(TagName=\"Weapon.Rifle.FireMode.SemiAuto\")")
        (bind _returnvalue (Class|ActionGameplayAbility|BatchRPCTryActivateAbility (Variables|Default|GetInstantAbilityHandle) true)) ; 일괄적으로 원격 어빌리티 활성화
        (if _returnvalue
          _
          (else
            _))
        (Ability|EndAbility)
        (else
          ;[1 1 1] 자동
          (if (== _firemode "(TagName=\"Weapon.Rifle.FireMode.FullAuto\")")
            (bind _returnvalue_2 (Class|ActionGameplayAbility|BatchRPCTryActivateAbility (Variables|Default|GetInstantAbilityHandle) false)) ; 일괄적으로 원격 어빌리티 활성화
            (if _returnvalue_2
              ;;[1 1 1] 버튼때면 어빌리티종료
              (Ability|Tasks|WaitInputRelease true
                (:then
                  ;;[1 1 1] 딜레이타임마다 남은총알 계산하고 계속 발사하기
                  (Ability|Tasks|WaitDelay (Variables|Default|GetTimeBetweenShots) :!label _label
                    (:OnFinish
                      (bind _returnvalue_3 (Class|GameplayAbility|CheckAbilityCost))
                      (if _returnvalue_3
                        (Default|FireBullet (Variables|Default|GetInstantAbility)) ; 총알 발사 함수
                        (goto _label)
                        (else
                          _)))))
                (:OnRelease
                  _))
              (Ability|EndAbility (Variables|Default|GetInstantAbility))
              (Ability|EndAbility)
              (else
                (Ability|EndAbility)))
            (else
              ;[1 1 1] 투사체
              (if (== (Variables|/Script/ActionWorldRPG.WeaponBase|GetFireMode (Variables|Default|GetSourceWeapon)) "(TagName=\"Weapon.Rifle.FireMode.Burst\")")
                (bind _returnvalue_4 (Class|ActionGameplayAbility|BatchRPCTryActivateAbility (Variables|Default|GetInstantAbilityHandle) false)) ; 일괄적으로 원격 어빌리티 활성화
                (if _returnvalue_4
                  (Ability|Tasks|WaitDelay (Variables|Default|GetTimeBetweenShots) ; 첫딜레이
                    (:OnFinish
                      (|RepeatAction (Variables|Default|GetTimeBetweenShots) 2 ; 2~3번째 딜레이
                        (:OnPerformAction
                          (bind _returnvalue_5 (Class|GameplayAbility|CheckAbilityCost))
                          (if _returnvalue_5
                            (Default|FireBullet (Variables|Default|GetInstantAbility))
                            (Development|PrintString "Burst")
                            (else
                              (Ability|EndAbility (Variables|Default|GetInstantAbility) :!label _label_2)
                              (Ability|EndAbility))))
                        (:OnFinished
                          (goto _label_2)))))
                  (else
                    (Ability|EndAbility)))
                (else
                  (Ability|EndAbility))))))))))

(fn CheckCost
  (params (Handle :type Gameplay%20Ability%20Spec%20Handle%20Structure) (ActorInfo :type Gameplay%20Ability%20Actor%20Info%20Structure%20%28by%20ref%29))
  (bind _abilitysystemcomponent (Utilities|Struct|BreakGameplayAbilityActorInfo ActorInfo))
  (bind _asb_weapon (Utilities|Casting|CastToB_Weapon (Class|ActionGameplayAbility|GetSourceObject Handle ActorInfo)))
  (if (and (or (>= (Class|WeaponBase|GetPrimaryClipAmmo _asb_weapon) (Variables|Default|GetAmmoCost)) (Class|WeaponBase|HasInfiniteAmmo _asb_weapon)) (|CallParentFunction Handle ActorInfo))
    (return true)
    (else
      ;[1 1 1] 탄약부족으로 인한 재장전
      (bind _returnvalue (Class|ActionBlueprintFunctionLibrary|IsPrimaryAbilityInstanceActive _abilitysystemcomponent Handle)) ; 총알을 못쏘는 상태인 딱 그 상태
      (if _returnvalue ; 여기서 True면 어빌리티는 활성화되어있지만 총알은없는상태
        _
        (else
          ;;[1 1 1] 리로드태그에 의한 어빌리티를 활성화
          (Abilities|TryActivateAbilitiesbyTag _abilitysystemcomponent (GameplayTags|MakeGameplayTagContainerfromArray (Utilities|Array|MakeArray "(TagName=\"Ability.Weapon.Reload\")")) true) ; 어빌리티도 비활성화이고 총알도 없는상태
        ))
      (return false))))