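; Rifle secondary-fire Gameplay Ability that provides hold-to-aim zoom on the player's camera.
; Activation caches the player and source weapon, applies an aiming effect and tweens to the weapon's zoom FOV.
; Input release tweens back to the default third-person FOV, applies an aiming-removal effect and ends the ability once reached.
; OnEndAbility ensures the removal effect was applied, removes both effects, ends both FOV tasks and snaps FOV to default.
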(event Ability|EventActivateAbility
  (Variables|Default|SetGE_AimingRemoval "")
  (Variables|Default|GetOwningPlayer
    (:then
      _)
    (:else
      (bind _asbp_player (Utilities|Casting|CastToBP_Player (Ability|GetAvatarActorfromActorInfo)))
      (Variables|Default|SetOwningPlayer _asbp_player)))
  (Variables|Default|GetSourceWeapon
    (:then
      _)
    (:else
      (bind _asb_weapon (Utilities|Casting|CastToB_Weapon (Ability|GetCurrentSourceObject)))
      (Variables|Default|SetSourceWeapon _asb_weapon)))
  (bind _returnvalue (Ability|ApplyGameplayEffectToOwner (Variables|Default|GetGE_Aiming_Class) (Ability|GetAbilityLevel)))
  (Variables|Default|SetGE_Aiming _returnvalue)
  ;[1 1 1] ZoomIn
  (bind _asynctaskproxy (|WaitChangeFOV "None" (Variables|/Script/ActionWorldRPG.PlayerBase|GetCameraComp (Variables|Default|GetOwningPlayer)) (Variables|/Script/ActionWorldRPG.WeaponBase|GetZoomFOV (Variables|Default|GetSourceWeapon)) 0.1)
    (:then
      (Variables|Default|SetZoomInTask _asynctaskproxy)
      (Ability|Tasks|WaitInputRelease true
        (:OnRelease
          ;[1 1 1] ZoomOut
          (bind _asynctaskproxy_2 (|WaitChangeFOV "None" (Variables|/Script/ActionWorldRPG.PlayerBase|GetCameraComp (Variables|Default|GetOwningPlayer)) (Variables|/Script/ActionWorldRPG.PlayerBase|GetDefault3PFOV (Variables|Default|GetOwningPlayer)) 0.07)
            (:then
              (Variables|Default|SetZoomOutTask _asynctaskproxy_2)
              ;[1 1 1] Apply Removal Effect
              (bind _returnvalue_2 (Ability|ApplyGameplayEffectToOwner (Variables|Default|GetGE_AimingRemoval_Class) (Ability|GetAbilityLevel)))
              (Variables|Default|SetGE_AimingRemoval _returnvalue_2))
            (:OnTargetFOVReached
              (Ability|EndAbility))))))))

(event Ability|EventOnEndAbility
  (params (bWasCancelled :type Boolean))
  (bind _owningplayer (Variables|Default|GetOwningPlayer))
  (bind _returnvalue (Ability|GameplayEffect|GetActiveGameplayEffectStackCount (Variables|Default|GetGE_AimingRemoval)))
  (if (> _returnvalue 0)
    _
    (else
      (bind _returnvalue_2 (Ability|ApplyGameplayEffectToOwner (Variables|Default|GetGE_AimingRemoval_Class) (Ability|GetAbilityLevel)))
      (Variables|Default|SetGE_AimingRemoval _returnvalue_2)))
  (Ability|RemoveGameplayEffectFromOwnerWithHandle (Variables|Default|GetGE_Aiming))
  (Ability|RemoveGameplayEffectFromOwnerWithHandle (Variables|Default|GetGE_AimingRemoval))
  (bind _zoomintask (Variables|Default|GetZoomInTask)
    (:then
      (GameplayTasks|EndTask _zoomintask))
    (:else
      _))
  (bind _zoomouttask (Variables|Default|GetZoomOutTask)
    (:then
      (GameplayTasks|EndTask _zoomouttask))
    (:else
      _))
  (Camera|SetFieldOfView (Variables|/Script/ActionWorldRPG.PlayerBase|GetCameraComp _owningplayer) (Variables|/Script/ActionWorldRPG.PlayerBase|GetDefault3PFOV _owningplayer)))