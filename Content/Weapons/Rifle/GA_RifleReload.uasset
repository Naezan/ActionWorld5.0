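; Rifle reload gameplay ability that refills the active equipment slot item's clip from spare ammo stored as stat tag stacks.
; Activation is allowed only when the clip is below capacity and spare rounds remain.
; It caches weapon, player and item, starts the reload montage, then immediately adds a loose reload tag and transfers ammo without waiting for an anim event.
; Montage completion ends the ability, interruption cancels it, and ending removes the tag.
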(event Ability|EventActivateAbility
  (Utilities|CheckandSetUpCacheables)
  (Development|PrintString "ReloadAction")
  (|PlayMontageandWaitforEvent "None" "/Game/Assets/Heavy_space_trooper/character/Animations/Actions/MM_Rifle_Reload_Montage.MM_Rifle_Reload_Montage" "(GameplayTags=((TagName=\"Ability.Weapon.Reload\")))" 1.0 "None" false 1.0
    (:then
      (Utilities|FlowControl|Sequence
        (:then_0
          (Ability|GameplayEffect|AddLooseGameplayTags (Ability|GetOwningActorfromActorInfo) (GameplayTags|MakeLiteralGameplayTagContainer "(GameplayTags=((TagName=\"Ability.Weapon.Reload\")))")))
        (:then_1
          (CallFunction|ReloadAmmo))))
    (:OnCompleted
      (Ability|EndAbility))
    (:OnInterrupted
      (Ability|CancelAbility :!label _label))
    (:OnCancelled
      (goto _label))))

(event Ability|EventOnEndAbility
  (params (bWasCancelled :type Boolean))
  (Ability|GameplayEffect|RemoveLooseGameplayTags (Ability|GetOwningActorfromActorInfo) (GameplayTags|MakeLiteralGameplayTagContainer "(GameplayTags=((TagName=\"Ability.Weapon.Reload\")))")))

(fn K2CanActivateAbility
  (params (ActorInfo :type Gameplay%20Ability%20Actor%20Info%20Structure) (Handle :type Gameplay%20Ability%20Spec%20Handle%20Structure))
  (bind _returnvalue (Class|EquipmentBarComponent|GetActiveSlotItem (Actor|GetComponentbyClass (.PlayerController (Utilities|Struct|BreakGameplayAbilityActorInfo ActorInfo)) "/Script/ActionWorldRPG.EquipmentBarComponent")))
  (Utilities|IsValid _returnvalue
    (:Is%20Valid
      (return "" (and (< (Class|InventoryItemInstance|GetStatTagStackCount _returnvalue "(TagName=\"Weapon.Ammo.Clip\")") (Class|InventoryItemInstance|GetStatTagStackCount _returnvalue "(TagName=\"Weapon.Ammo.ClipSize\")")) (> (Class|InventoryItemInstance|GetStatTagStackCount _returnvalue "(TagName=\"Weapon.Ammo.Spare\")") 0))))
    (:Is%20Not%20Valid
      (return "" false))))

(fn ReloadAmmo
  (bind _currentiteminstance (Variables|Default|GetCurrentItemInstance))
  (bind _returnvalue (Class|InventoryItemInstance|GetStatTagStackCount _currentiteminstance "(TagName=\"Weapon.Ammo.Spare\")"))
  (bind _output_get (Variables|Default|SetAmountWeWantToReload (- (Class|InventoryItemInstance|GetStatTagStackCount _currentiteminstance "(TagName=\"Weapon.Ammo.ClipSize\")") (Class|InventoryItemInstance|GetStatTagStackCount _currentiteminstance "(TagName=\"Weapon.Ammo.Clip\")"))))
  (if (<= _output_get _returnvalue) ; 탄창과 남은탄창간의 조건비교
    (Variables|Default|SetAmountWeCanReload _output_get)
    (else
      (Variables|Default|SetAmountWeCanReload _returnvalue)))
  (Class|InventoryItemInstance|AddStatTagStack (Variables|Default|GetCurrentItemInstance) "(TagName=\"Weapon.Ammo.Clip\")" (Variables|Default|GetAmountWeCanReload))
  (Class|InventoryItemInstance|RemoveStatTagStack (Variables|Default|GetCurrentItemInstance) "(TagName=\"Weapon.Ammo.Spare\")" (Variables|Default|GetAmountWeCanReload)))