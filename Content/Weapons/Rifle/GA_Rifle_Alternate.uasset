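; Gameplay ability for the rifle's alternate action that cycles its fire mode from Burst to FullAuto to SemiAuto and back to Burst.
; On activation it caches the B_Rifle source object and the player controller, branches on the current fire mode tag, and writes the next mode and its status text onto the rifle.
; The ability then ends; the final controller validity check drives no logic.
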(event Ability|EventActivateAbility
  (Variables|Default|GetWeaponRifle
    (:then
      _)
    (:else
      (bind _asb_rifle (Utilities|Casting|CastToB_Rifle (Ability|GetCurrentSourceObject)))
      (Variables|Default|SetWeaponRifle _asb_rifle)))
  (Variables|Default|GetPlayerController
    (:then
      _)
    (:else
      (bind _asaction_player_controller (Utilities|Casting|CastToActionPlayerController (.playercontroller (Ability|GetActorInfo)))
        (:then
          (Variables|Default|SetPlayerController _asaction_player_controller))
        (:CastFailed
          _))))
  (if (== (Variables|/Script/ActionWorldRPG.WeaponBase|GetFireMode (Variables|Default|GetWeaponRifle)) "(TagName=\"Weapon.Rifle.FireMode.Burst\")")
    (Variables|/Script/ActionWorldRPG.WeaponBase|SetFireMode (Variables|Default|GetWeaponRifle) "(TagName=\"Weapon.Rifle.FireMode.FullAuto\")")
    (Variables|/Script/ActionWorldRPG.WeaponBase|SetStatusText (Variables|Default|GetWeaponRifle) (Variables|Default|GetFullAutoStatus))
    (Variables|Default|GetPlayerController :!label _label
      (:then
        _)
      (:else
        _))
    (Ability|EndAbility)
    (elif (== (Variables|/Script/ActionWorldRPG.WeaponBase|GetFireMode (Variables|Default|GetWeaponRifle)) "(TagName=\"Weapon.Rifle.FireMode.FullAuto\")")
      (Variables|/Script/ActionWorldRPG.WeaponBase|SetFireMode (Variables|Default|GetWeaponRifle) "(TagName=\"Weapon.Rifle.FireMode.SemiAuto\")")
      (Variables|/Script/ActionWorldRPG.WeaponBase|SetStatusText (Variables|Default|GetWeaponRifle) (Variables|Default|GetSemiAutoStatus))
      (goto _label)
      (elif (== (Variables|/Script/ActionWorldRPG.WeaponBase|GetFireMode (Variables|Default|GetWeaponRifle)) "(TagName=\"Weapon.Rifle.FireMode.SemiAuto\")")
        (Variables|/Script/ActionWorldRPG.WeaponBase|SetFireMode (Variables|Default|GetWeaponRifle) "(TagName=\"Weapon.Rifle.FireMode.Burst\")")
        (Variables|/Script/ActionWorldRPG.WeaponBase|SetStatusText (Variables|Default|GetWeaponRifle) (Variables|Default|GetBurstStatus))
        (goto _label)))))