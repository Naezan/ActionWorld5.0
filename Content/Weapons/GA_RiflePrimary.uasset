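; Rifle primary-fire Gameplay Ability that drives semi-auto, full-auto and burst modes, read from the source weapon.
; It caches the weapon and GA_RiflePrimaryInstant's handle and instance, then activates that ability through a batched RPC after a short delay.
; Semi-auto ends immediately.
; Full-auto and burst call FireBullet at shot intervals while cost checks pass, until input release or two repeats respectively, then end both abilities.
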(event Ability|EventActivateAbility
  (bind _sourceweapon (Variables|Default|GetSourceWeapon))
  (bind _firemode (Variables|/Script/ActionWorldRPG.WeaponBase|GetFireMode _sourceweapon))
  (Utilities|CheckandSetUpCacheables)
  (Ability|Tasks|WaitDelay 0.03
    (:OnFinish
      ;[1 1 1] 반자동
      (if (== _firemode "(TagName=\"Weapon.Rifle.FireMode.SemiAuto\")")
        (bind _returnvalue (Class|ActionGameplayAbility|BatchRPCTryActivateAbility (Variables|Default|GetInstantAbilityHandle) true)) ; 일괄적으로 원격 어빌리티 활성화
        (if _returnvalue
          _
          (else
            _))
        (Ability|EndAbility)
        (else
          ;[1 1 1] 자동
          (if (== _firemode "(TagName=\"Weapon.Rifle.FireMode.FullAuto\")")
            (bind _returnvalue_2 (Class|ActionGameplayAbility|BatchRPCTryActivateAbility (Variables|Default|GetInstantAbilityHandle) false)) ; 일괄적으로 원격 어빌리티 활성화
            (if _returnvalue_2
              ;;[1 1 1] 버튼때면 어빌리티종료
              (Ability|Tasks|WaitInputRelease true
                (:then
                  ;;[1 1 1] 딜레이타임마다 남은총알 계산하고 계속 발사하기
                  (Ability|Tasks|WaitDelay (Variables|Default|GetTimeBetweenShots) :!label _label
                    (:OnFinish
                      (bind _returnvalue_3 (Class|GameplayAbility|CheckAbilityCost))
                      (if _returnvalue_3
                        (Default|FireBullet (Variables|Default|GetInstantAbility)) ; 총알 발사 함수
                        (goto _label)
                        (else
                          _)))))
                (:OnRelease
                  _))
              (Ability|EndAbility (Variables|Default|GetInstantAbility))
              (Ability|EndAbility)
              (else
                (Ability|EndAbility)))
            (else
              ;[1 1 1] 투사체
              (if (== (Variables|/Script/ActionWorldRPG.WeaponBase|GetFireMode (Variables|Default|GetSourceWeapon)) "(TagName=\"Weapon.Rifle.FireMode.Burst\")")
                (bind _returnvalue_4 (Class|ActionGameplayAbility|BatchRPCTryActivateAbility (Variables|Default|GetInstantAbilityHandle) false)) ; 일괄적으로 원격 어빌리티 활성화
                (if _returnvalue_4
                  (Ability|Tasks|WaitDelay (Variables|Default|GetTimeBetweenShots) ; 첫딜레이
                    (:OnFinish
                      (|RepeatAction (Variables|Default|GetTimeBetweenShots) 2 ; 2~3번째 딜레이
                        (:OnPerformAction
                          (bind _returnvalue_5 (Class|GameplayAbility|CheckAbilityCost))
                          (if _returnvalue_5
                            (Default|FireBullet (Variables|Default|GetInstantAbility))
                            (Development|PrintString "Burst")
                            (else
                              (Ability|EndAbility (Variables|Default|GetInstantAbility) :!label _label_2)
                              (Ability|EndAbility))))
                        (:OnFinished
                          (goto _label_2)))))
                  (else
                    (Ability|EndAbility)))
                (else
                  (Ability|EndAbility))))))))))